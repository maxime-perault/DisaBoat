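; BP_ocean builds an endless-looking ocean from a grid of BP_water_tile actors that follows the player character.
; The construction script spawns the tiles as child actor components, centred on the actor.
; Each tick, once the character's root moves over a tile's size along X or Y, the trailing row or column jumps to the leading edge, recycling tiles instead of spawning new ones.
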(event `self.ReceiveBeginPlay`
  (set `self.z_root` (.z (`SceneComponent.K2_GetComponentLocation` (`self.DefaultSceneRoot`))))
  (bind _asthird_person_character (cast `/Game/ThirdPersonBP/Blueprints/ThirdPersonCharacter` (`GameplayStatics.GetPlayerCharacter` 0)))
  (set `self.start_location` (`SceneComponent.K2_GetComponentLocation` (`/Game/ThirdPersonBP/Blueprints/ThirdPersonCharacter.Boat` _asthird_person_character)))
  (set `self.boat` _asthird_person_character))

(event `self.ReceiveTick`
  (params (DeltaSeconds :type "Float (single-precision)"))
  (bind _y (.y (`self.start_location`)))
  (bind _x (.x (`self.start_location`)))
  (bind _y_2 (.y (`SceneComponent.K2_GetComponentLocation` (`Actor.RootComponent` (`self.boat`)))))
  (bind _x_2 (.x (`SceneComponent.K2_GetComponentLocation` (`Actor.RootComponent` (`self.boat`)))))
  (bind _returnvalue (> (`KismetMathLibrary.Abs` (- _x_2 _x)) (`self.tile_size`)))
  (bind _returnvalue_2 (> (`KismetMathLibrary.Abs` (- _y_2 _y)) (`self.tile_size`)))
  (if (and _returnvalue (< _x_2 _x))
    ;[1 1 1] X < 0
    (for _array_element (`SceneComponent.GetChildrenComponents` (`self.DefaultSceneRoot`) false)
      (if (== (.x (`SceneComponent.RelativeLocation` _array_element)) (+ (`self.x`) (* (`self.tile_size`) (- (`self.x_size_tiles`) 1.0))))
        (`SceneComponent.K2_SetRelativeLocation` _array_element (`KismetMathLibrary.MakeVector` (- (`self.x`) (`self.tile_size`)) (.y (`SceneComponent.RelativeLocation` _array_element)) (.z (`SceneComponent.RelativeLocation` _array_element))) false false)))
    (set `self.x` (- (`self.x`) (`self.tile_size`)))
    (set `self.start_location` (`KismetMathLibrary.MakeVector` (.x (`SceneComponent.K2_GetComponentLocation` (`Actor.RootComponent` (`self.boat`)))) (.y (`self.start_location`)) (.z (`self.start_location`))))
    (else
      ;[1 1 1] X > 0
      (if (and _returnvalue (> _x_2 _x))
        (for _array_element_2 (`SceneComponent.GetChildrenComponents` (`self.DefaultSceneRoot`) false)
          (if (== (.x (`SceneComponent.RelativeLocation` _array_element_2)) (`self.x`))
            (`SceneComponent.K2_SetRelativeLocation` _array_element_2 (`KismetMathLibrary.MakeVector` (+ (`self.x`) (* (`self.tile_size`) (`self.x_size_tiles`))) (.y (`SceneComponent.RelativeLocation` _array_element_2)) (.z (`SceneComponent.RelativeLocation` _array_element_2))) false false)))
        (set `self.x` (+ (`self.x`) (`self.tile_size`)))
        (set `self.start_location` (`KismetMathLibrary.MakeVector` (.x (`SceneComponent.K2_GetComponentLocation` (`Actor.RootComponent` (`self.boat`)))) (.y (`self.start_location`)) (.z (`self.start_location`)))))))
  (if (and _returnvalue_2 (< _y_2 _y))
    ;[1 1 1] Y < 0
    (for _array_element_3 (`SceneComponent.GetChildrenComponents` (`self.DefaultSceneRoot`) false)
      (if (== (.y (`SceneComponent.RelativeLocation` _array_element_3)) (+ (`self.y`) (* (`self.tile_size`) (- (`self.y_size_tiles`) 1.0))))
        (`SceneComponent.K2_SetRelativeLocation` _array_element_3 (`KismetMathLibrary.MakeVector` (.x (`SceneComponent.RelativeLocation` _array_element_3)) (- (`self.y`) (`self.tile_size`)) (.z (`SceneComponent.RelativeLocation` _array_element_3))) false false)))
    (set `self.y` (- (`self.y`) (`self.tile_size`)))
    (set `self.start_location` (`KismetMathLibrary.MakeVector` (.x (`self.start_location`)) (.y (`SceneComponent.K2_GetComponentLocation` (`Actor.RootComponent` (`self.boat`)))) (.z (`self.start_location`))))
    (else
      ;[1 1 1] Y > 0
      (if (and _returnvalue_2 (> _y_2 _y))
        (for _array_element_4 (`SceneComponent.GetChildrenComponents` (`self.DefaultSceneRoot`) false)
          (if (== (.y (`SceneComponent.RelativeLocation` _array_element_4)) (`self.y`))
            (`SceneComponent.K2_SetRelativeLocation` _array_element_4 (`KismetMathLibrary.MakeVector` (.x (`SceneComponent.RelativeLocation` _array_element_4)) (+ (`self.y`) (* (`self.tile_size`) (`self.y_size_tiles`))) (.z (`SceneComponent.RelativeLocation` _array_element_4))) false false)))
        (set `self.y` (+ (`self.y`) (`self.tile_size`)))
        (set `self.start_location` (`KismetMathLibrary.MakeVector` (.x (`self.start_location`)) (.y (`SceneComponent.K2_GetComponentLocation` (`Actor.RootComponent` (`self.boat`)))) (.z (`self.start_location`))))))))

(fn `UserConstructionScript`
  ;[1 1 1] Start position for X and Y
  (set `self.x` (- 0.0 (/ (* (- (`self.x_size_tiles`) 1.0) (`self.tile_size`)) 2.0)))
  (set `self.y` (- 0.0 (/ (* (- (`self.y_size_tiles`) 1.0) (`self.tile_size`)) 2.0)))
  (while (< (`self.y_array`) (`self.y_size_tiles`))
    (set `self.x_array` 0.0)
    (while (< (`self.x_array`) (`self.x_size_tiles`))
      (bind _returnvalue (`AddComponent|NODE_AddChildActorComponent-1` :`RelativeTransform` (`KismetMathLibrary.MakeTransform` (`KismetMathLibrary.MakeVector` (+ (`self.x`) (* (`self.x_array`) (`self.tile_size`))) (+ (`self.y`) (* (`self.y_array`) (`self.tile_size`)))))))
      (`ChildActorComponent.SetChildActorClass` _returnvalue "/Game/WaterBP/BP_water_tile.BP_water_tile_C")
      (cast `/Game/WaterBP/BP_water_tile` (`ChildActorComponent.ChildActor` _returnvalue))
      (`/Engine/EditorBlueprintResources/StandardMacros.IncrementFloat` (`self.x_array`)))
    (`/Engine/EditorBlueprintResources/StandardMacros.IncrementFloat` (`self.y_array`))))