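; ObstaclesLineBP is an actor that spawns a patterned row of obstacles along world Y, centered on its location.
; On BeginPlay it walks the ObstaclesLine array and spawns an Obstacle at each enabled slot, leaving gaps elsewhere.
; Slots are evenly spaced, with a half-step shift to center even-sized lines.
; Spawned obstacles are tracked in an array and destroyed along with the line actor.
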(event `self.ReceiveBeginPlay`
  (set `self.SpawnBegin` (`KismetMathLibrary.MakeVector` (.x (`self.K2_GetActorLocation`)) (- (.y (`self.K2_GetActorLocation`)) (* (/ (`self.LineSize`) 2) (`self.DistanceBetweenObstacles`))) (.z (`self.K2_GetActorLocation`))))
  (if (not (> (`KismetMathLibrary.FMod` (`KismetMathLibrary.Conv_IntToDouble` (`self.LineSize`)) 2.0) 0.0))
    (set `self.SpawnBegin` (`KismetMathLibrary.MakeVector` (.x (`self.SpawnBegin`)) (+ (.y (`self.SpawnBegin`)) (/ (`self.DistanceBetweenObstacles`) 2.0)) (.z (`self.SpawnBegin`)))))
  (while (< (`self.i`) (`self.LineSize`))
    (if (`|GetArrayItem` (`self.ObstaclesLine`) (`self.i`))
      (bind _returnvalue (`|SpawnActorFromClass` "/Game/ObstaclesBP/Obstacle.Obstacle_C" (`KismetMathLibrary.MakeTransform` (`KismetMathLibrary.MakeVector` (.x (`self.SpawnBegin`)) (+ (.y (`self.SpawnBegin`)) (* (`self.i`) (`self.DistanceBetweenObstacles`))) (.z (`self.SpawnBegin`)))) "Undefined" "OverrideRootScale" null null))
      (`KismetArrayLibrary.Array_Add` (`self.Obstacles`) _returnvalue))
    (`/Engine/EditorBlueprintResources/StandardMacros.IncrementInt` (`self.i`))))

(event `self.ReceiveDestroyed`
  (for _array_element (`self.Obstacles`)
    (`self.K2_DestroyActor` _array_element)))

(fn `UserConstructionScript`
  (set `self.ObstaclesLine` (`self.ObstaclesLine`)))